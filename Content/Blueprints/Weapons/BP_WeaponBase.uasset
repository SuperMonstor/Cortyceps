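; Base hitscan weapon for the FPS player, handling firing, magazine and reserve ammo, and reloading.
; WeaponFire decrements ammo, then spawns an impact effect actor with the hit result from CalculateShot's camera-forward line trace, randomly offset for spread.
; The muzzle socket is passed but unused in the trace.
; Ammo checks are separate functions; reload overwrites the magazine from reserve, discarding rounds left in it.
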(event `self.ReceiveBeginPlay`
  (bind _asfps_character (cast `/Game/Blueprints/FPS_character` (`GameplayStatics.GetPlayerPawn` 0)))
  (set `self.PlayerRef` _asfps_character))

(fn `CalculateShot`
  (params (Camera :type "CameraComponent Object Reference") (WeaponMesh :type "SceneComponent Object Reference") (WeaponFireSocketName :type Name))
  (returns (HitResult :type "HitResult Structure"))
  (locals (LocalCamera :type "CameraComponent Object Reference") (LocalSocketName :type "SceneComponent Object Reference") (NewLocalVar_0 :type Name))
  (bind _bulletspread (`self.BulletSpread`))
  (bind (_returnvalue_location _returnvalue_rotation) (`KismetMathLibrary.BreakTransform` (`SceneComponent.K2_GetComponentToWorld` (`local.LocalCamera`))))
  (bind _returnvalue (* _bulletspread -1.0))
  (`|ExecutionSequence`
    (:`then_0`
      (set `local.LocalCamera` Camera)
      (set `local.LocalSocketName` WeaponMesh)
      (set `local.NewLocalVar_0` WeaponFireSocketName))
    (:`then_1`
      (bind _outhit (`KismetSystemLibrary.LineTraceSingleForObjects` _returnvalue_location (`KismetMathLibrary.MakeVector` (+ (.x (+ _returnvalue_location (* (`KismetMathLibrary.GetForwardVector` _returnvalue_rotation) (`self.LineTraceDistance`)))) (`KismetMathLibrary.RandomFloatInRange` _returnvalue _bulletspread)) (+ (.y (+ _returnvalue_location (* (`KismetMathLibrary.GetForwardVector` _returnvalue_rotation) (`self.LineTraceDistance`)))) (`KismetMathLibrary.RandomFloatInRange` _returnvalue _bulletspread)) (+ (.z (+ _returnvalue_location (* (`KismetMathLibrary.GetForwardVector` _returnvalue_rotation) (`self.LineTraceDistance`)))) (`KismetMathLibrary.RandomFloatInRange` _returnvalue _bulletspread))) (`|MakeArray` "ObjectTypeQuery1" "ObjectTypeQuery2" :!type "EObjectTypeQuery Enum") false (`|MakeArray` (`GameplayStatics.GetPlayerPawn` 0) :!type "Actor Object Reference")))
      (return _outhit))))

(fn `hasAmmoInMag`
  (returns (hasAmmo :type Boolean) (isMagFull :type Boolean))
  (return (> (`self.CurrentAmmo`) 0) (== (`self.CurrentAmmo`) (`self.MaxMagAmmo`))))

(fn `hasExtraAmmo`
  (returns (hasExtraAmmo :type Boolean))
  (return (> (`self.CurrentTotalAmmo`) 0)))

(fn `UserConstructionScript`)

(fn `WeaponFire`
  (set `self.CurrentAmmo` (- (`self.CurrentAmmo`) 1))
  (bind _hitresult (`self.CalculateShot` (`/Game/Blueprints/FPS_character.Camera` (`self.PlayerRef`)) (`self.GunMesh`) "MuzzleFlash"))
  (bind (_bblockinghit _binitialoverlap _time _distance _location _impactpoint) (`GameplayStatics.BreakHitResult` _hitresult))
  (`|SpawnActorFromClass` (`self.ImpactEffectClass`) (`KismetMathLibrary.MakeTransform` _impactpoint) "Undefined" "OverrideRootScale" null _hitresult _bblockinghit null))

(fn `WeaponReload`
  (bind _returnvalue (`KismetMathLibrary.Min` (`self.MaxMagAmmo`) (`self.CurrentTotalAmmo`)))
  (set `self.CurrentAmmo` _returnvalue)
  (set `self.CurrentTotalAmmo` (- (`self.CurrentTotalAmmo`) _returnvalue)))